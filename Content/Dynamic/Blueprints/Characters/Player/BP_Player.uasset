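; BP_Player is a player character that moves along the world X axis, flipping control yaw to face its travel direction.
; Enhanced Input drives move, jump and sprint, with sprint speed applied only while grounded.
; GroundBox overlaps track grounding and restore rising gravity on contact.
; Releasing jump or falling switches to a separate downward gravity scale to shape the jump arc, and Tick prints falling-state debug text.
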(event OnComponentEndOverlap(GroundBox)
  (params (OverlappedComponent :type Primitive%20Component%20Object%20Reference) (OtherActor :type Actor%20Object%20Reference) (OtherComp :type Primitive%20Component%20Object%20Reference) (OtherBodyIndex :type Integer))
  (Variables|Default|SetIsGrounded false)
  (Development|PrintString "off ground"))

(event OnComponentBeginOverlap(GroundBox)
  (params (OverlappedComponent :type Primitive%20Component%20Object%20Reference) (OtherActor :type Actor%20Object%20Reference) (OtherComp :type Primitive%20Component%20Object%20Reference) (OtherBodyIndex :type Integer) (bFromSweep :type Boolean) (SweepResult :type Hit%20Result%20Structure%20%28by%20ref%29))
  (Variables|Default|SetIsGrounded true)
  (Variables|/Script/Engine.CharacterMovementComponent|SetGravityScale (Variables|Character|GetCharacterMovement) (Variables|Default|GetJumpGravityUp)))

(event Input|EnhancedActionEvents|EnhancedInputActionIA_Jump
  (params (ActionValue :type Boolean) (ElapsedSeconds :type Float%20%28double-precision%29) (TriggeredSeconds :type Float%20%28double-precision%29) (InputAction :type Input%20Action%20Object%20Reference :default "/Game/Dynamic/Inputs/Actions/IA_Jump.IA_Jump"))
  (:Triggered
    (Character|Jump))
  (:Canceled
    (Character|StopJumping :!label _label)
    (Variables|/Script/Engine.CharacterMovementComponent|SetGravityScale (Variables|Character|GetCharacterMovement) (Variables|Default|GetJumpGravityDown)))
  (:Completed
    (goto _label)))

(event Input|EnhancedActionEvents|EnhancedInputActionIA_Move
  (params (ActionValue :type Float%20%28double-precision%29) (ElapsedSeconds :type Float%20%28double-precision%29) (TriggeredSeconds :type Float%20%28double-precision%29) (InputAction :type Input%20Action%20Object%20Reference :default "/Game/Dynamic/Inputs/Actions/IA_Move.IA_Move"))
  (Pawn|Input|AddMovementInput "1.000000,0.000000,0.000000" ActionValue false)
  (CallFunction|UpdateRotation ActionValue))

(event Input|EnhancedActionEvents|EnhancedInputActionIA_Sprint
  (params (ActionValue :type Boolean) (ElapsedSeconds :type Float%20%28double-precision%29) (TriggeredSeconds :type Float%20%28double-precision%29) (InputAction :type Input%20Action%20Object%20Reference :default "/Game/Dynamic/Inputs/Actions/IA_Sprint.IA_Sprint"))
  (:Triggered
    (if (Variables|Default|GetIsGrounded)
      (Variables|/Script/Engine.CharacterMovementComponent|SetMaxWalkSpeed (Variables|Character|GetCharacterMovement) (Variables|Default|GetSprintSpeed))))
  (:Completed
    (Variables|/Script/Engine.CharacterMovementComponent|SetMaxWalkSpeed (Variables|Character|GetCharacterMovement) (Variables|Default|GetWalkSpeed))))

(event EventBeginPlay
  (|CallParentFunction)
  (bind _asplayer_controller (Utilities|Casting|CastToPlayerController (Pawn|GetController)))
  (Input|AddMappingContext (PlayerController|LocalPlayerSubsystems|GetEnhancedInputLocalPlayerSubsystem _asplayer_controller) "/Game/Dynamic/Inputs/IMC_Action.IMC_Action" 0 "(bIgnoreAllPressedKeysUntilRelease=True,bForceImmediately=False,bNotifyUserSettings=False)"))

(event EventTick
  (params (DeltaSeconds :type Float%20%28single-precision%29))
  (if (< (.z (Transformation|GetVelocity)) -1.0)
    (Variables|Default|SetIsFalling true)
    (Variables|/Script/Engine.CharacterMovementComponent|SetGravityScale (Variables|Character|GetCharacterMovement) (Variables|Default|GetJumpGravityDown))
    (Development|PrintString "FALLING" true true "(R=1.000000,G=0.077638,B=0.000000,A=1.000000)")
    (else
      (Variables|Default|SetIsFalling false)
      (Development|PrintString "NOT FALLING" true true "(R=0.000000,G=1.000000,B=0.214649,A=1.000000)"))))

(fn ConstructionScript
  (|CallParentFunction))

(fn UpdateRotation
  (params (Direction :type Float%20%28double-precision%29))
  (Pawn|SetControlRotation (Pawn|GetController) (select (>= Direction 0.0) (Math|Rotator|MakeRotator 0.0 0.0 0.0) (Math|Rotator|MakeRotator 0.0 0.0 1.8e+02))))